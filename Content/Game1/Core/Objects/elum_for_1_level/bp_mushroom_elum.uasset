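; Glowing mushroom light source that tells dryad and third-person characters whether they are in its light.
; BeginPlay sets the point light's color and radius and sizes three trigger spheres from the light radius and nearest-position distance.
; Entering the outer sphere turns on the character's light flag and leaving the slightly smaller one clears it, also registering this actor on the dryad.
; Re-entering inner spheres restores the flag: middle for third-person, nearest for dryad.
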(event `self.ReceiveBeginPlay`
  (bind _radius_of_light (`self.radius_of_light`))
  (`LightComponent.SetLightColor` (`self.PointLight1`) (`KismetMathLibrary.Conv_ColorToLinearColor` (`self.Light Color`)) true)
  (`SphereComponent.SetSphereRadius` (`self.Sphere`) _radius_of_light true)
  (`SphereComponent.SetSphereRadius` (`self.Sphere1`) (- _radius_of_light 100.0) true)
  (`SphereComponent.SetSphereRadius` (`self.Sphere2`) (`self.nearest_position_of_light`) true)
  (`LocalLightComponent.SetAttenuationRadius` (`self.PointLight1`) (`self.radius_of_light`)))

(event `self.Sphere.OnComponentBeginOverlap`
  (params (OverlappedComponent :type "PrimitiveComponent Object Reference") (OtherActor :type "Actor Object Reference") (OtherComp :type "PrimitiveComponent Object Reference") (OtherBodyIndex :type Integer) (bFromSweep :type Boolean) (SweepResult :type "HitResult Structure (by ref)"))
  (`|ExecutionSequence`
    (:`then_0`
      (bind _asbpchar_driada (cast `/Game/Game1/Core/Objects/driada/BPCHAR_driada` OtherActor))
      (set `/Game/Game1/Core/Objects/driada/BPCHAR_driada.is_Light_turn_on` true _asbpchar_driada)
      (set `/Game/Game1/Core/Objects/driada/BPCHAR_driada.actual_light` self _asbpchar_driada))
    (:`then_1`
      (bind _asbp_third_person_character (cast `/Game/Game1/Core/Characters/BP_ThirdPersonCharacter` OtherActor))
      (set `/Game/Game1/Core/Characters/BP_ThirdPersonCharacter.light_turn_on` true _asbp_third_person_character)
      (`KismetSystemLibrary.PrintString` "true"))))

(event `self.Sphere1.OnComponentEndOverlap`
  (params (OverlappedComponent :type "PrimitiveComponent Object Reference") (OtherActor :type "Actor Object Reference") (OtherComp :type "PrimitiveComponent Object Reference") (OtherBodyIndex :type Integer))
  (`|ExecutionSequence`
    (:`then_0`
      (bind _asbpchar_driada (cast `/Game/Game1/Core/Objects/driada/BPCHAR_driada` OtherActor))
      (set `/Game/Game1/Core/Objects/driada/BPCHAR_driada.is_Light_turn_on` false _asbpchar_driada)
      (set `/Game/Game1/Core/Objects/driada/BPCHAR_driada.actual_light` self _asbpchar_driada))
    (:`then_1`
      (bind _asbp_third_person_character (cast `/Game/Game1/Core/Characters/BP_ThirdPersonCharacter` OtherActor))
      (set `/Game/Game1/Core/Characters/BP_ThirdPersonCharacter.light_turn_on` false _asbp_third_person_character)
      (`KismetSystemLibrary.PrintString` "false"))))

(event `self.Sphere1.OnComponentBeginOverlap`
  (params (OverlappedComponent :type "PrimitiveComponent Object Reference") (OtherActor :type "Actor Object Reference") (OtherComp :type "PrimitiveComponent Object Reference") (OtherBodyIndex :type Integer) (bFromSweep :type Boolean) (SweepResult :type "HitResult Structure (by ref)"))
  (bind _asbp_third_person_character (cast `/Game/Game1/Core/Characters/BP_ThirdPersonCharacter` OtherActor))
  (set `/Game/Game1/Core/Characters/BP_ThirdPersonCharacter.light_turn_on` true _asbp_third_person_character))

(event `self.Sphere2.OnComponentBeginOverlap`
  (params (OverlappedComponent :type "PrimitiveComponent Object Reference") (OtherActor :type "Actor Object Reference") (OtherComp :type "PrimitiveComponent Object Reference") (OtherBodyIndex :type Integer) (bFromSweep :type Boolean) (SweepResult :type "HitResult Structure (by ref)"))
  (bind _asbpchar_driada (cast `/Game/Game1/Core/Objects/driada/BPCHAR_driada` OtherActor))
  (set `/Game/Game1/Core/Objects/driada/BPCHAR_driada.is_Light_turn_on` true _asbpchar_driada))

(fn `UserConstructionScript`)