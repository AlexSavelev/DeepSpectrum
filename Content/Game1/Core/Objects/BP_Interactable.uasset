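; Base interactable actor that lets the player trigger an action with the Interact input while standing in its box trigger, meant for child actors to override OnInteract.
; Player overlap enables input, opens a gate and shows the character's InteractWidget with an inscription formatted with the bound key name; leaving reverses this.
; Interact release calls OnInteract if 3D input is allowed and the gate is open.
; The construction script sizes and raises the trigger from TriggerSize.
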(event `self.ReceiveBeginPlay`
  ;[1 1 1] Format Inscription
  (bind _returnvalue (`/Game/Game1/Core/Functional/BPFL_Main.GetKeyDisplayNames` "Interact"))
  (set `self.FormatedInscription` (`|FormatText` (`self.Inscription`) (select `int` (`KismetMathLibrary.Conv_BoolToInt` (!= (`KismetArrayLibrary.Array_Length` _returnvalue) 0)) :`0` "???" :`1` (`|GetArrayItem` _returnvalue)))))

(event `InputAction|Interact`
  (params (Key :type "Key Structure"))
  ;[1 1 1] Input Registration
  (:`Released`
    (`/Game/Game1/Core/Functional/BPML_Actor.IsInput3DAllowed`
      (:`Yes`
        (`/Engine/EditorBlueprintResources/StandardMacros.Gate` true :!label _label
          (:`Exit`
            (`self.OnInteract`)))))))

(event `self.BoxTrigger.OnComponentBeginOverlap`
  (params (OverlappedComponent :type "PrimitiveComponent Object Reference") (OtherActor :type "Actor Object Reference") (OtherComp :type "PrimitiveComponent Object Reference") (OtherBodyIndex :type Integer) (bFromSweep :type Boolean) (SweepResult :type "HitResult Structure (by ref)"))
  (bind _interactwidget (`/Game/Game1/Core/Characters/BP_ThirdPersonCharacter.InteractWidget` (`/Game/Game1/Core/Functional/BPFL_Main.GetTPPCharacter`)))
  ;[1 1 1] Input Registration
  (if (== OtherActor (`GameplayStatics.GetPlayerCharacter` 0))
    (`self.EnableInput` (`GameplayStatics.GetPlayerController` 0))
    (`TextBlock.SetText` (`/Game/Game1/Core/Widgets/WBP_Interact.InteractTextBlock` _interactwidget) (`self.FormatedInscription`))
    (`UserWidget.AddToViewport` _interactwidget 0)
    (goto _label :!via `Open`)))

(event `self.BoxTrigger.OnComponentEndOverlap`
  (params (OverlappedComponent :type "PrimitiveComponent Object Reference") (OtherActor :type "Actor Object Reference") (OtherComp :type "PrimitiveComponent Object Reference") (OtherBodyIndex :type Integer))
  ;[1 1 1] Input Registration
  (if (== OtherActor (`GameplayStatics.GetPlayerCharacter` 0))
    (`self.DisableInput` (`GameplayStatics.GetPlayerController` 0))
    (`Widget.RemoveFromParent` (`/Game/Game1/Core/Characters/BP_ThirdPersonCharacter.InteractWidget` (`/Game/Game1/Core/Functional/BPFL_Main.GetTPPCharacter`)))
    (goto _label :!via `Close`)))

(event `OnInteract`
  ;[1 1 1] On Interact
  (`KismetSystemLibrary.PrintString` "It`s the base Interactable Object. Create child actors to fill the content"))

(fn `UserConstructionScript`
  (bind _triggersize (`self.TriggerSize`))
  (`BoxComponent.SetBoxExtent` (`self.BoxTrigger`) _triggersize true)
  (`SceneComponent.K2_SetRelativeLocation` (`self.BoxTrigger`) (`KismetMathLibrary.MakeVector` 0.0 0.0 (.z _triggersize)) false false))