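; BP_Programmable is a base actor for interactable objects that the player programs, meant to be extended by child actors.
; Interacting switches input to interface mode and fires the OnProgram event.
; The base OnProgram only prints a placeholder message, then calls OnFinishProgramming, which restores 3D input.
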(event `self.OnInteract`
  (`/Game/Game1/Core/Functional/BPFL_Main.SetInputInterface`)
  (`self.OnProgram`))

(event `OnProgram`
  ;[1 1 1] Programming
  (`KismetSystemLibrary.PrintString` "It`s the base Programming Object. Create child actors to fill the content")
  (`self.OnFinishProgramming`))

(event `OnFinishProgramming`
  ;[1 1 1] Programming
  (`/Game/Game1/Core/Functional/BPFL_Main.SetInput3D`))

(fn `UserConstructionScript`
  (`parent.UserConstructionScript`))