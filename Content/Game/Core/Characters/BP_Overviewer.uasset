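; Overview-phase player actor that pans a camera along a spline so the player can select and program objects before play.
; MoveRight offsets it on Y, then snaps it to the BP_CameraSpline found on every axis event, not the CameraSpline stored by Setup.
; OverviewInteract release line-traces under the mouse to open BP_Programmable editing, locking interaction and Play until finished.
; The overview widget's Play button removes it and calls Manager.SetGMPlayer.
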(event `self.ReceiveBeginPlay`
  (bind _returnvalue (`|CreateWidget` "/Game/Game/Core/Objects/Programmable/Widgets/WB_POProgram.WB_POProgram_C"))
  (set `self.ProgrammingWidget` _returnvalue)
  (bind _returnvalue_2 (`|CreateWidget` "/Game/Game/Core/Objects/Programmable/Widgets/WB_Overview.WB_Overview_C"))
  (bind _output_get (set `self.OverviewWidget` _returnvalue_2))
  (add `Button.OnClicked` (`/Game/Game/Core/Objects/Programmable/Widgets/WB_Overview.PlayBtn` _output_get) (delegate `OnPlay`)))

(event `OnPlay`
  (if (not (`self.bInEditor`))
    (`Widget.RemoveFromParent` (`self.OverviewWidget`))
    (`/Game/Game/Core/Objects/BP_ProgrammingManager.SetGMPlayer` (`self.Manager`))))

(event `InputAxis|MoveRight` :overrideparent false
  (params (AxisValue :type "Float (single-precision)"))
  (`self.K2_AddActorWorldOffset` (`KismetMathLibrary.MakeVector` 0.0 (* AxisValue (`self.Speed`))))
  ;[1 1 1] Spline Attachment
  (bind _outactors (`GameplayStatics.GetAllActorsOfClass` "/Game/Game/Core/Cameras/BP_CameraSpline.BP_CameraSpline_C"))
  (bind _cameralocation (`/Game/Game/Core/Cameras/BP_CameraSpline.CalculateCameraLocation` (`|GetArrayItem` _outactors) (`self.K2_GetActorLocation`)))
  (`self.K2_SetActorLocation` _cameralocation))

(event `OnOverview`
  (`UserWidget.AddToViewport` (`self.OverviewWidget`) 0))

(event `InputAction|OverviewInteract`
  (params (Key :type "Key Structure"))
  (:`Released`
    (if (not (`self.bInEditor`))
      (bind (_returnvalue _outhit) (`/Game/Game/Core/Functional/BPFL_Main.MouseLineTrace` (`self.TraceLength`)))
      (if _returnvalue
        (bind (_bblockinghit _binitialoverlap _time _distance _location _impactpoint _normal _impactnormal _physmat _hitactor) (`GameplayStatics.BreakHitResult` _outhit))
        (if (`KismetMathLibrary.ClassIsChildOf` (`GameplayStatics.GetObjectClass` _hitactor) "/Game/Game/Core/Objects/Programmable/BP_Programmable.BP_Programmable_C")
          (bind _asbp_programmable (cast `/Game/Game/Core/Objects/Programmable/BP_Programmable` _hitactor :!pure true))
          (`/Game/Game/Core/Objects/Programmable/BP_Programmable.OnProgram` _asbp_programmable)
          (add `/Game/Game/Core/Objects/Programmable/BP_Programmable.OnFinishProgramming` _asbp_programmable (delegate `OnFinishProgramming`))
          (set `self.bInEditor` true))))))

(event `OnFinishProgramming`
  (set `self.bInEditor` false))

(fn `Setup`
  (params (Spline :type "/Game/Game/Core/Cameras/BP_CameraSpline Object Reference") (Speed :type "Float (double-precision)") (TraceLength :type "Float (double-precision)") (Location :type "Vector Structure"))
  (set `self.CameraSpline` Spline)
  (set `self.Speed` Speed)
  (set `self.TraceLength` TraceLength)
  (`self.K2_SetActorLocation` Location)
  (return))

(fn `UserConstructionScript`)