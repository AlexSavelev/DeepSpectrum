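; BP_MainMenuPawn is the main menu pawn, handling startup logo playback and menu input setup.
; On BeginPlay it creates and stores the WB_MM widget, switches input to UI-only and shows the mouse cursor.
; It spawns a BP_LogoManager with LogosSequence, starts the logos, then binds ShowMenu to their finish event.
; ShowMenu only destroys the logo manager; the widget is never added to the viewport here.
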(event `self.ReceiveBeginPlay`
  (bind _returnvalue (`GameplayStatics.GetPlayerController` 0))
  (bind _returnvalue_2 (`|CreateWidget` "/Game/Game/Core/MainMenu/Widgets/WB_MM.WB_MM_C"))
  (set `self.MainWidgetRef` _returnvalue_2)
  (`WidgetBlueprintLibrary.SetInputMode_UIOnlyEx` _returnvalue null)
  (set `PlayerController.bShowMouseCursor` true _returnvalue)
  (bind _returnvalue_3 (`|SpawnActorFromClass` "/Game/Game/Core/MainMenu/SubClasses/BP_LogoManager.BP_LogoManager_C" (`KismetMathLibrary.MakeTransform` (0.0 0.0 0.0)) "Undefined" "OverrideRootScale" null (`self.LogosSequence`) null))
  (set `self.LogosManager` _returnvalue_3)
  (`/Game/Game/Core/MainMenu/SubClasses/BP_LogoManager.ShowAllLogos` _returnvalue_3)
  (add `/Game/Game/Core/MainMenu/SubClasses/BP_LogoManager.OnFinishShow` _returnvalue_3 (delegate `ShowMenu`)))

(event `ShowMenu`
  (`self.K2_DestroyActor` (`self.LogosManager`)))

(fn `UserConstructionScript`)