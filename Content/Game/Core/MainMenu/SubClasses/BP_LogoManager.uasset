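; BP_LogoManager plays a sequence of logo screens for the main menu, each an image on black or a video, with optional 2D audio.
; It creates a WB_MM_Logo widget on BeginPlay, and ShowAllLogos displays and focuses it to start the sequence.
; A custom ForSequence loop advances whenever the widget reports it has finished.
; After the last entry, it removes the widget and fires the OnFinishShow dispatcher.
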(event `self.ReceiveBeginPlay`
  (bind _returnvalue (`|CreateWidget` "/Game/Game/Core/MainMenu/Widgets/WB_MM_Logo.WB_MM_Logo_C"))
  (bind _output_get (set `self.Widget` _returnvalue))
  (add `/Game/Game/Core/MainMenu/Widgets/WB_MM_Logo.OnFinish` _output_get (delegate `OnLogoFinish`)))

(event `OnLogoFinish`
  (bind _widget (`self.Widget`))
  (bind (_type _media _audio) (`self.ForSequence` :!label _label)
    (:`then`
      (`/Engine/EditorBlueprintResources/StandardMacros.IsValid` _audio
        (:`Is Valid`
          (`GameplayStatics.PlaySound2D` _audio 1.0 1.0 0.0 null null))
        (:`Is Not Valid`
          _))
      (switch `/Game/Game/Core/MainMenu/SubClasses/E_MM_LogoType` _type
        (:`NewEnumerator0`
          (`/Game/Game/Core/MainMenu/Widgets/WB_MM_Logo.ShowImage` _widget (cast `Texture2D` _media :!pure true) (struct :`A` 1.0)))
        (:`NewEnumerator1`
          (`/Game/Game/Core/MainMenu/Widgets/WB_MM_Logo.ShowVideo` _widget (cast `MediaSource` _media :!pure true)))))
    (:`Finish`
      (`Widget.RemoveFromParent` (`self.Widget`))
      (`self.OnFinishShow`))))

(event `ShowAllLogos`
  (bind _widget (`self.Widget`))
  (`UserWidget.AddToViewport` _widget 10)
  (`Widget.SetFocus` _widget)
  (goto _label :!via `execute`))

(fn `UserConstructionScript`)