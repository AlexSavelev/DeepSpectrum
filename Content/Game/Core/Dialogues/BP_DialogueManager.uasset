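; Manager that plays a single dialogue on BeginPlay, chosen by DialogueID from the DT_Dialogues data table.
; It creates a WB_Dialogue widget, adds it to the viewport with focus and listens for its OnFinishImg event.
; A ForDialogue macro acts as an event-driven iterator over the row's Objectives, advancing each time the widget reports finishing.
; When the entries run out, it removes the widget and fires OnFinish.
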(event `self.ReceiveBeginPlay`
  (`self.ParceDialogue`)
  (bind _returnvalue (`|CreateWidget` "/Game/Game/Core/Dialogues/Widgets/WB_Dialogue.WB_Dialogue_C"))
  (bind _output_get (set `self.Widget` _returnvalue))
  (add `/Game/Game/Core/Dialogues/Widgets/WB_Dialogue.OnFinishImg` _output_get (delegate `FinishImg`))
  (`self.ShowDialogue`))

(event `FinishImg`
  (bind _objective (`self.ForDialogue` :!label _label)
    (:`then`
      (`/Game/Game/Core/Dialogues/Widgets/WB_Dialogue.OnShowObj` (`self.Widget`) _objective))
    (:`Finish`
      (`Widget.RemoveFromParent` (`self.Widget`))
      (`self.OnFinish`))))

(event `ShowDialogue`
  (bind _widget (`self.Widget`))
  (`UserWidget.AddToViewport` _widget 10)
  (`Widget.SetFocus` _widget)
  (goto _label :!via `execute`))

(fn `ParceDialogue`
  (bind _returnvalue (`|GetDataTableRow` "/Game/Game/Core/Dialogues/DT_Dialogues.DT_Dialogues" (`self.DialogueID`))
    (:`then`
      (set `self.Dialogue` _returnvalue)
      (return))))

(fn `UserConstructionScript`)