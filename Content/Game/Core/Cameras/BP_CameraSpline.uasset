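; Camera rail actor that maps an actor's location to a camera position along an authored spline.
; Construction copies the spline's points with locations filtered by GuideAxis, and BeginPlay spawns a BP_RuntimeSpline from them as a navigation spline.
; CalculateCameraLocation finds the navigation spline key closest to the filtered actor location, clamps it to a minimum, and samples the original spline there in world space.
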(event `self.ReceiveBeginPlay`
  (bind _returnvalue (`|SpawnActorFromClass` "/Game/Game/Core/Cameras/BP_RuntimeSpline.BP_RuntimeSpline_C" (`self.GetTransform`) "Undefined" "OverrideRootScale" self (`self.Points`) null))
  (set `self.NavigationSpline` (`/Game/Game/Core/Cameras/BP_RuntimeSpline.Spline` _returnvalue)))

(fn `CalculateCameraLocation`
  (params (ActorLocation :type "Vector Structure"))
  (returns (CameraLocation :type "Vector Structure"))
  (return (`SplineComponent.GetLocationAtSplineInputKey` (`self.Spline`) (`KismetMathLibrary.FMax` (`SplineComponent.FindInputKeyClosestToWorldLocation` (`self.NavigationSpline`) (`/Game/Game/Core/Functional/BPML_Main.FilterVector` ActorLocation (`self.GuideAxis`))) 2.0) "World")))

(fn `UserConstructionScript`
  (bind _spline (`self.Spline`))
  (`KismetArrayLibrary.Array_Clear` (`self.Points`))
  (for _index (range (`SplineComponent.GetNumberOfSplinePoints` _spline))
    (bind (_returnvalue_location _returnvalue_rotation _returnvalue_scale) (`KismetMathLibrary.BreakTransform` (`SplineComponent.GetTransformAtSplinePoint` _spline _index "Local" false)))
    (`KismetArrayLibrary.Array_Add` (`self.Points`) (make `SplinePoint` (`KismetMathLibrary.Conv_IntToDouble` _index) (`/Game/Game/Core/Functional/BPML_Main.FilterVector` _returnvalue_location (`self.GuideAxis`)) (`SplineComponent.GetArriveTangentAtSplinePoint` _spline _index "Local") (`SplineComponent.GetLeaveTangentAtSplinePoint` _spline _index "Local") _returnvalue_rotation _returnvalue_scale (`SplineComponent.GetSplinePointType` _spline _index)))))