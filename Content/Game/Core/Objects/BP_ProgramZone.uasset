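; BP_ProgramZone is a trigger volume that marks a programming zone in the level.
; On BeginPlay it finds and caches the BP_ProgrammingManager actor.
; When the player character overlaps its box, it passes its overviewer spline, speed, trace length and own location to the manager's SetGMOverviewer.
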(event `self.ReceiveBeginPlay`
  (bind _returnvalue (`GameplayStatics.GetActorOfClass` "/Game/Game/Core/Objects/BP_ProgrammingManager.BP_ProgrammingManager_C"))
  (set `self.Manager` _returnvalue))

(event `self.Box.OnComponentBeginOverlap`
  (params (OverlappedComponent :type "PrimitiveComponent Object Reference") (OtherActor :type "Actor Object Reference") (OtherComp :type "PrimitiveComponent Object Reference") (OtherBodyIndex :type Integer) (bFromSweep :type Boolean) (SweepResult :type "HitResult Structure (by ref)"))
  (if (== OtherActor (`GameplayStatics.GetPlayerCharacter` 0))
    (`/Game/Game/Core/Objects/BP_ProgrammingManager.SetGMOverviewer` (`self.Manager`) (`self.OverviewersSpline`) (`self.OverviewersSpeed`) (`self.OverviewersTraceLength`) (`self.K2_GetActorLocation`))))

(fn `UserConstructionScript`)