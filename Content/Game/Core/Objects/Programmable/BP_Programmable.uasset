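; Base actor for world objects the player can reprogram, with stub events for overview mode, player mode and updates.
; The construction script looks up the object's description by Name, seeding missing programs with their first script and filling missing per-script limits.
; OnProgram opens the pawn's WB_POProgram widget, which returns edited programs through a bound callback that triggers OnUpdate.
; Helpers toggle custom-depth highlighting and test player overlap.
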(event `OnProgram`
  (bind _aswb_poprogram (cast `/Game/Game/Core/Objects/Programmable/Widgets/WB_POProgram` (`/Game/Game/Core/Characters/BP_Overviewer.ProgrammingWidget` (`/Game/Game/Core/Functional/BPFL_Main.GetOVPawn`)) :!pure true))
  ;[1 1 1] Programming
  (`UserWidget.AddToViewport` _aswb_poprogram 0)
  (add `/Game/Game/Core/Objects/Programmable/Widgets/WB_POProgram.OnFinish` _aswb_poprogram (delegate `OnInterfaceFinished`))
  (`/Game/Game/Core/Objects/Programmable/Widgets/WB_POProgram.ProgramIt` _aswb_poprogram (`self.Name`) (`self.Programs`) (`self.Limits`)))

(event `OnInterfaceFinished`
  (params (NewPrograms :type "/Game/Game/Core/Objects/Programmable/Structs/Data/S_POData Structure"))
  (bind _aswb_poprogram (cast `/Game/Game/Core/Objects/Programmable/Widgets/WB_POProgram` (`/Game/Game/Core/Characters/BP_Overviewer.ProgrammingWidget` (`/Game/Game/Core/Functional/BPFL_Main.GetOVPawn`)) :!pure true))
  ;[1 1 1] Programming
  (set `self.Programs` NewPrograms)
  (`Widget.RemoveFromParent` _aswb_poprogram)
  (remove `/Game/Game/Core/Objects/Programmable/Widgets/WB_POProgram.OnFinish` _aswb_poprogram (delegate `OnInterfaceFinished`))
  (`self.OnFinishProgramming`)
  (`self.OnUpdate`))

(event `self.ReceiveBeginPlay`
  (bind _returnvalue (`GameplayStatics.GetActorOfClass` "/Game/Game/Core/Objects/BP_PlayerManager.BP_PlayerManager_C"))
  (add `/Game/Game/Core/Objects/BP_PlayerManager.OnChangeGameModeOverview` _returnvalue (delegate `BindedOverview`))
  (add `/Game/Game/Core/Objects/BP_PlayerManager.OnChangeGameModePlayer` _returnvalue (delegate `BindedPlayer`))
  (`self.OnUpdate`)
  (`self.Player`))

(event `BindedOverview`
  (`self.Overview`))

(event `BindedPlayer`
  (`self.Player`))

(event `Overview`)

(event `Player`)

(event `OnUpdate`
  (`KismetSystemLibrary.PrintString` "Updated"))

(fn `FillScriptLimitsInfo`
  (params (Scripts :type "Array of /Game/Game/Core/Objects/Programmable/Structs/Desc/S_POScriptDesc Structure"))
  (returns (Limits :type "/Game/Game/Core/Objects/Programmable/Structs/Limits/S_POProgramLimits Structure"))
  (locals (SL :type "Map of Name to /Game/Game/Core/Objects/Programmable/Structs/Limits/S_POScriptLimit Structure"))
  (for _array_element Scripts
    (bind (_name _displayname _argument _argumentplaceholder _icon _defaultlimits) (break `/Game/Game/Core/Objects/Programmable/Structs/Desc/S_POScriptDesc` _array_element))
    (`BlueprintMapLibrary.Map_Add` (`local.SL`) _name _defaultlimits))
  (return (make `/Game/Game/Core/Objects/Programmable/Structs/Limits/S_POProgramLimits` (`local.SL`))))

(fn `HasActorOverlapping`
  (params (Collision :type "PrimitiveComponent Object Reference"))
  (returns (ReturnValue :type Boolean))
  (return (`KismetArrayLibrary.Array_Contains` (`PrimitiveComponent.GetOverlappingActors` Collision "/Script/Engine.Pawn") (`GameplayStatics.GetPlayerPawn` 0))))

(fn `SetHighlightEnabled`
  (params (IsEnabled :type Boolean))
  (for _array_element (`self.K2_GetComponentsByClass` "/Script/Engine.PrimitiveComponent")
    (`PrimitiveComponent.SetRenderCustomDepth` _array_element IsEnabled))
  (return))

(fn `UserConstructionScript`
  (bind _programs_programs (break `/Game/Game/Core/Objects/Programmable/Structs/Data/S_POData` (`self.Programs`)))
  (bind _limits_programs (break `/Game/Game/Core/Objects/Programmable/Structs/Limits/S_POLimits` (`self.Limits`)))
  (bind _desc (`/Game/Game/Core/Objects/Programmable/FLBP_Programmable.GetObjectDescription` (`self.Name`)))
  (bind _item (`/Game/Game/Core/Functional/BPML_Main.ForEachLoopWithContinue` (`.Programs_7_2C2B0DB9465AE70329F4B6AAA3E2CF94` (break `/Game/Game/Core/Objects/Programmable/Structs/Desc/S_PODesc` _desc)) :!via `execute` :!label _label)
    (:`then`
      (bind (_name _displayname _scripts) (break `/Game/Game/Core/Objects/Programmable/Structs/Desc/S_POProgramDesc` _item))
      (if (not (`BlueprintMapLibrary.Map_Contains` _programs_programs _name))
        (bind (_output_name _output_displayname _output_argument _output_argumentplaceholder _output_icon _output_defaultlimits) (break `/Game/Game/Core/Objects/Programmable/Structs/Desc/S_POScriptDesc` (`|GetArrayItem` _scripts)))
        (`BlueprintMapLibrary.Map_Add` _programs_programs _name (make `/Game/Game/Core/Objects/Programmable/Structs/Data/S_POScript` _output_name (`KismetTextLibrary.Conv_StringToText` (select `/Game/Game/Core/Objects/Programmable/Structs/E_POScriptAdditionalArgument` _output_argument :`NewEnumerator1` (`KismetStringLibrary.Conv_IntToString` (`.Min_9_2471AA124284CD00A5B27BBC4009C766` (break `/Game/Game/Core/Objects/Programmable/Structs/Limits/S_POScriptLimit` _output_defaultlimits))))))))
      (if (`BlueprintMapLibrary.Map_Contains` _limits_programs _name)
        (goto _label)
        (else
          (`BlueprintMapLibrary.Map_Add` _limits_programs _name (`self.FillScriptLimitsInfo` _scripts))
          (goto _label))))))