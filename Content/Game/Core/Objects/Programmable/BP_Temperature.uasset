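; BP_Temperature is a programmable object that changes the player character's temperature, either fixing it or shifting it up or down.
; Its Programs map supplies Condition and Change scripts with numeric arguments, cached on update.
; In Player mode, Always activates immediately, while Time toggles on an interval and Distance follows player range via Tick, which Overview disables.
; Despite its name, GetHorizontalDistance measures full 3D distance.
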(event `self.OnUpdate`
  (bind _programs_programs (break `/Game/Game/Core/Objects/Programmable/Structs/Data/S_POData` (`self.Programs`)))
  (bind _value (`BlueprintMapLibrary.Map_Find` _programs_programs "Change"))
  (bind _value_2 (`BlueprintMapLibrary.Map_Find` _programs_programs "Condition"))
  ;[1 1 1] Setup
  (set `self.Condition` (break `/Game/Game/Core/Objects/Programmable/Structs/Data/S_POScript` _value_2))
  (set `self.ConditionValue` (`KismetMathLibrary.Conv_IntToDouble` (`KismetStringLibrary.Conv_StringToInt` (`KismetTextLibrary.Conv_TextToString` (`.Argument_9_554FC57544DA74CD8B7190AAC4106B00` (break `/Game/Game/Core/Objects/Programmable/Structs/Data/S_POScript` _value_2))))))
  (set `self.Change` (break `/Game/Game/Core/Objects/Programmable/Structs/Data/S_POScript` _value))
  (set `self.ChangeValue` (`KismetStringLibrary.Conv_StringToInt` (`KismetTextLibrary.Conv_TextToString` (`.Argument_9_554FC57544DA74CD8B7190AAC4106B00` (break `/Game/Game/Core/Objects/Programmable/Structs/Data/S_POScript` _value))))))

(event `Activate`
  (set `self.bActivated` true)
  (bind _asbp_third_person_character (cast `/Game/Game/Core/Characters/BP_ThirdPersonCharacter` (`GameplayStatics.GetPlayerPawn` 0)))
  (`/Game/Game/Core/Characters/BP_ThirdPersonCharacter.ChangeTemperature` _asbp_third_person_character (== (`self.Change`) "Fix") (select `bool` (== (`self.Change`) "Down") :`false` (`self.ChangeValue`) :`true` (* (`self.ChangeValue`) -1))))

(event `Deactivate`
  (set `self.bActivated` false)
  (bind _asbp_third_person_character (cast `/Game/Game/Core/Characters/BP_ThirdPersonCharacter` (`GameplayStatics.GetPlayerPawn` 0)))
  (`/Game/Game/Core/Characters/BP_ThirdPersonCharacter.ChangeTemperature` _asbp_third_person_character false 0))

(event `self.Player`
  (set `self.bPlayerIn` false)
  (set `self.bActivated` false)
  (if (== (`self.Condition`) "Always")
    (`self.SetActorTickEnabled` false)
    (`self.Activate`)
    (else
      (`self.SetActorTickEnabled` true))))

(event `self.Overview`
  (`self.SetActorTickEnabled` false))

(event `self.ReceiveTick`
  (params (DeltaSeconds :type "Float (single-precision)"))
  (bind _returnvalue (`self.GetHorizontalDistance`))
  (bind _returnvalue_2 (* 100 (`self.ConditionValue`)))
  ;[1 1 1] Check Conditions
  (switch `name` (`self.Condition`)
    (:`Time`
      (set `self.TimeTicked` (+ DeltaSeconds (`self.TimeTicked`)))
      (if (>= (`self.TimeTicked`) (`self.ConditionValue`))
        (set `self.TimeTicked` 0.0)
        (if (`self.bActivated`)
          (`self.Deactivate`)
          (else
            (`self.Activate`)))))
    (:`Distance`
      (if (`self.bActivated`)
        (if (> _returnvalue _returnvalue_2)
          (`self.Deactivate`))
        (elif (<= _returnvalue _returnvalue_2)
          (`self.Activate`))))))

(fn `GetHorizontalDistance`
  (returns (ReturnValue :type "Float (double-precision)"))
  (return (`KismetMathLibrary.VSize` (- (`self.K2_GetActorLocation`) (`self.K2_GetActorLocation` (`GameplayStatics.GetPlayerPawn` 0))))))

(fn `UserConstructionScript`
  (`parent.UserConstructionScript`))