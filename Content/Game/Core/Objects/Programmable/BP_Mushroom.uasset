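; Programmable mushroom that grows taller when its condition is met and can act as a trampoline for the player.
; OnUpdate reads the Condition, Size and Properties programs; Player mode starts ticking to evaluate Always, timed or player-distance conditions, while Overview stops it.
; Activate stretches the cube vertically, counter-scales the trigger and binds the bounce, which reverses fall speed up to a cap.
; Deactivate resets actor scale, not the cube's, and unbinds the bounce.
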(event `self.ReceiveBeginPlay`
  (set `self.start_scale` (`SceneComponent.K2_GetComponentScale` (`self.Cube`)))
  (`parent.ReceiveBeginPlay`))

(event `self.OnUpdate`
  (bind _programs (break `/Game/Game/Core/Objects/Programmable/Structs/Data/S_POData` (`self.Programs`)))
  (bind _value (`BlueprintMapLibrary.Map_Find` _programs "Condition"))
  ;[1 1 1] Parce Programs
  (set `self.Condition` (break `/Game/Game/Core/Objects/Programmable/Structs/Data/S_POScript` _value))
  (set `self.ConditionArg` (`KismetStringLibrary.Conv_StringToInt` (`KismetTextLibrary.Conv_TextToString` (`.Argument_9_554FC57544DA74CD8B7190AAC4106B00` (break `/Game/Game/Core/Objects/Programmable/Structs/Data/S_POScript` _value)))))
  (set `self.SizeChangePercent` (`KismetStringLibrary.Conv_StringToInt` (`KismetTextLibrary.Conv_TextToString` (`.Argument_9_554FC57544DA74CD8B7190AAC4106B00` (break `/Game/Game/Core/Objects/Programmable/Structs/Data/S_POScript` (`BlueprintMapLibrary.Map_Find` _programs "Size"))))))
  (set `self.Properties` (break `/Game/Game/Core/Objects/Programmable/Structs/Data/S_POScript` (`BlueprintMapLibrary.Map_Find` _programs "Properties"))))

(event `mushroom_reset`)

(event `Activate`
  (bind (_returnvalue_x _returnvalue_y) (`KismetMathLibrary.BreakVector` (`SceneComponent.K2_GetComponentScale` (`self.Cube`))))
  (bind _returnvalue (* (`KismetMathLibrary.Conv_IntToDouble` (`self.SizeChangePercent`)) 2.0))
  (`SceneComponent.SetWorldScale3D` (`self.Cube`) (`KismetMathLibrary.MakeVector` _returnvalue_x _returnvalue_y _returnvalue))
  (`SceneComponent.SetWorldScale3D` (`self.TrampolineTrigger`) (`KismetMathLibrary.MakeVector` 5.0 5.0 (/ 0.5 _returnvalue)))
  ;[1 1 1] Activation & Deactivation
  (if (== (`self.Properties`) "Trampoline")
    (add `PrimitiveComponent.OnComponentBeginOverlap` (`self.TrampolineTrigger`) (delegate `OnTranpolineOverlap`))))

(event `self.Player`
  (`self.SetActorTickEnabled` true)
  (set `self.TimeTicked` 0.0)
  (if (== (`self.Condition`) "Always")
    (set `self.bMetCondition` true)
    (`self.Activate`)
    (else
      (set `self.bMetCondition` false)
      (`self.Deactivate`))))

(event `self.Overview`
  (`self.SetActorTickEnabled` false))

(event `OnTranpolineOverlap`
  (params (OverlappedComponent :type "PrimitiveComponent Object Reference") (OtherActor :type "Actor Object Reference") (OtherComp :type "PrimitiveComponent Object Reference") (OtherBodyIndex :type Integer) (bFromSweep :type Boolean) (SweepResult :type "HitResult Structure (by ref)"))
  (bind _returnvalue (`GameplayStatics.GetPlayerCharacter` 0))
  (bind (_returnvalue_x _returnvalue_y _returnvalue_z) (`KismetMathLibrary.BreakVector` (`self.GetVelocity` _returnvalue)))
  ;[1 1 1] Activation & Deactivation
  (`KismetSystemLibrary.PrintString` "Hello")
  (if (== OtherActor _returnvalue)
    (`Character.LaunchCharacter` _returnvalue (`KismetMathLibrary.MakeVector` (* _returnvalue_x 0.8) (* _returnvalue_y 0.8) (`KismetMathLibrary.FMin` (* _returnvalue_z -2.1) (`self.max_jump`))) true true)))

(event `Deactivate`
  ;[1 1 1] Activation & Deactivation
  (`self.SetActorScale3D` (1.0 1.0 1.0))
  (if (== (`self.Properties`) "Trampoline")
    (remove `PrimitiveComponent.OnComponentBeginOverlap` (`self.TrampolineTrigger`) (delegate `OnTranpolineOverlap`))))

(event `self.ReceiveTick`
  (params (DeltaSeconds :type "Float (single-precision)"))
  (bind _returnvalue (`self.GetPlayerHorizontalDistance`))
  (bind _returnvalue_2 (* 100 (`KismetMathLibrary.Conv_IntToDouble` (`self.ConditionArg`))))
  ;[1 1 1] Check Conditions
  (switch `name` (`self.Condition`)
    (:`Time`
      (set `self.TimeTicked` (+ DeltaSeconds (`self.TimeTicked`)))
      (if (`self.bMetCondition`)
        (if (>= (`self.TimeTicked`) 1.0)
          (set `self.TimeTicked` 0.0)
          (set `self.bMetCondition` false)
          (`self.Deactivate`))
        (elif (>= (`self.TimeTicked`) (`KismetMathLibrary.Conv_IntToDouble` (`self.ConditionArg`)))
          (set `self.TimeTicked` 0.0)
          (set `self.bMetCondition` true)
          (`self.Activate`))))
    (:`Distance`
      (if (`self.bMetCondition`)
        (if (> _returnvalue _returnvalue_2)
          (set `self.bMetCondition` false)
          (`self.Deactivate`))
        (elif (<= _returnvalue _returnvalue_2)
          (set `self.bMetCondition` true)
          (`self.Activate`))))))

(event `self.TrampolineTrigger.OnComponentBeginOverlap`
  (params (OverlappedComponent :type "PrimitiveComponent Object Reference") (OtherActor :type "Actor Object Reference") (OtherComp :type "PrimitiveComponent Object Reference") (OtherBodyIndex :type Integer) (bFromSweep :type Boolean) (SweepResult :type "HitResult Structure (by ref)"))
  (if true
    _))

(fn `GetPlayerHorizontalDistance`
  (returns (ReturnValue :type "Float (double-precision)"))
  (bind (_returnvalue_x _returnvalue_y) (`KismetMathLibrary.BreakVector` (`self.K2_GetActorLocation`)))
  (bind (_returnvalue_x_2 _returnvalue_y_2) (`KismetMathLibrary.BreakVector` (`self.K2_GetActorLocation` (`GameplayStatics.GetPlayerPawn` 0))))
  (return (`KismetMathLibrary.Distance2D` (`KismetMathLibrary.MakeVector2D` _returnvalue_x _returnvalue_y) (`KismetMathLibrary.MakeVector2D` _returnvalue_x_2 _returnvalue_y_2))))

(fn `UserConstructionScript`
  (`parent.UserConstructionScript`))