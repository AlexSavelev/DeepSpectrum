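; BP_Geyser is a programmable geyser object that takes its settings from its Programs map.
; On each OnUpdate event it looks up program entries by name: the State script sets Enabled, and Condition supplies a script plus an integer argument.
; Power and Size come from their entries' arguments converted to integers.
; The graph only caches these values, with no eruption logic and an empty construction script.
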(event `self.OnUpdate`
  (bind _programs_programs (break `/Game/Game/Core/Objects/Programmable/Structs/Data/S_POData` (`self.Programs`)))
  (bind _value (`BlueprintMapLibrary.Map_Find` _programs_programs "Condition"))
  (set `self.bEnabled` (== (break `/Game/Game/Core/Objects/Programmable/Structs/Data/S_POScript` (`BlueprintMapLibrary.Map_Find` _programs_programs "State")) "Enabled"))
  (set `self.Condition` (break `/Game/Game/Core/Objects/Programmable/Structs/Data/S_POScript` _value))
  (set `self.ConditionArg` (`KismetStringLibrary.Conv_StringToInt` (`KismetTextLibrary.Conv_TextToString` (`.Argument_9_554FC57544DA74CD8B7190AAC4106B00` (break `/Game/Game/Core/Objects/Programmable/Structs/Data/S_POScript` _value)))))
  (set `self.Power` (`KismetStringLibrary.Conv_StringToInt` (`KismetTextLibrary.Conv_TextToString` (`.Argument_9_554FC57544DA74CD8B7190AAC4106B00` (break `/Game/Game/Core/Objects/Programmable/Structs/Data/S_POScript` (`BlueprintMapLibrary.Map_Find` _programs_programs "Power"))))))
  (set `self.Size` (`KismetStringLibrary.Conv_StringToInt` (`KismetTextLibrary.Conv_TextToString` (`.Argument_9_554FC57544DA74CD8B7190AAC4106B00` (break `/Game/Game/Core/Objects/Programmable/Structs/Data/S_POScript` (`BlueprintMapLibrary.Map_Find` _programs_programs "Size")))))))

(fn `UserConstructionScript`)