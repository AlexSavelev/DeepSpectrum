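; Tutorial programmable cube that resizes according to its assigned Condition and Size programs.
; OnUpdate parses the programs, Player enables ticking and immediately applies an Always condition, and Overview stops ticking.
; Tick handles Time (timed delay, one-second pulse) and Distance (player's horizontal range) conditions.
; Activation scales the SCube component by Size, while deactivation resets actor scale to one, leaving saved StartScale and parsed Properties unused.
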(event `self.ReceiveBeginPlay`
  (set `self.start_scale` (`SceneComponent.K2_GetComponentScale` (`self.S_Cube`)))
  (`parent.ReceiveBeginPlay`))

(event `self.OnUpdate`
  (bind _programs (break `/Game/Game/Core/Objects/Programmable/Structs/Data/S_POData` (`self.Programs`)))
  (bind _value (`BlueprintMapLibrary.Map_Find` _programs "Condition"))
  ;[1 1 1] Parce Programs
  (set `self.Condition` (break `/Game/Game/Core/Objects/Programmable/Structs/Data/S_POScript` _value))
  (set `self.ConditionArg` (`KismetStringLibrary.Conv_StringToInt` (`KismetTextLibrary.Conv_TextToString` (`.Argument_9_554FC57544DA74CD8B7190AAC4106B00` (break `/Game/Game/Core/Objects/Programmable/Structs/Data/S_POScript` _value)))))
  (set `self.SizeChangePercent` (`KismetStringLibrary.Conv_StringToInt` (`KismetTextLibrary.Conv_TextToString` (`.Argument_9_554FC57544DA74CD8B7190AAC4106B00` (break `/Game/Game/Core/Objects/Programmable/Structs/Data/S_POScript` (`BlueprintMapLibrary.Map_Find` _programs "Size"))))))
  (set `self.Properties` (break `/Game/Game/Core/Objects/Programmable/Structs/Data/S_POScript` (`BlueprintMapLibrary.Map_Find` _programs "Properties"))))

(event `mushroom_reset`)

(event `AVtivate`
  (bind _returnvalue (`KismetMathLibrary.Conv_IntToDouble` (`self.SizeChangePercent`)))
  (`SceneComponent.SetWorldScale3D` (`self.S_Cube`) (`KismetMathLibrary.MakeVector` (* _returnvalue 0.2) (* _returnvalue 0.2 1.0) (* (`KismetMathLibrary.Conv_IntToDouble` (`self.SizeChangePercent`)) 0.2))))

(event `self.Player`
  (`self.SetActorTickEnabled` true)
  (set `self.TimeTicked` 0.0)
  (if (== (`self.Condition`) "Always")
    (set `self.bMetCondition` true)
    (`self.AVtivate`)
    (else
      (set `self.bMetCondition` false)
      (`self.deactiv`))))

(event `self.Overview`
  (`self.SetActorTickEnabled` false))

(event `deactiv`
  ;[1 1 1] Activation & Deactivation
  (`self.SetActorScale3D` (1.0 1.0 1.0)))

(event `self.ReceiveTick`
  (params (DeltaSeconds :type "Float (single-precision)"))
  (bind _returnvalue (`self.GetPlayerHorizontalDistance_0`))
  (bind _returnvalue_2 (* 100 (`KismetMathLibrary.Conv_IntToDouble` (`self.ConditionArg`))))
  ;[1 1 1] Check Conditions
  (switch `name` (`self.Condition`)
    (:`Time`
      (set `self.TimeTicked` (+ DeltaSeconds (`self.TimeTicked`)))
      (if (`self.bMetCondition`)
        (if (>= (`self.TimeTicked`) 1.0)
          (set `self.TimeTicked` 0.0)
          (set `self.bMetCondition` false)
          (`self.deactiv`))
        (elif (>= (`self.TimeTicked`) (`KismetMathLibrary.Conv_IntToDouble` (`self.ConditionArg`)))
          (set `self.TimeTicked` 0.0)
          (set `self.bMetCondition` true)
          (`self.AVtivate`))))
    (:`Distance`
      (if (`self.bMetCondition`)
        (if (> _returnvalue _returnvalue_2)
          (set `self.bMetCondition` false)
          (`KismetSystemLibrary.PrintString` "Hello1")
          (`self.deactiv`))
        (elif (<= _returnvalue _returnvalue_2)
          (set `self.bMetCondition` true)
          (`KismetSystemLibrary.PrintString` "2")
          (`self.AVtivate`))))))

(event `Deactivate`)

(fn `Activate`)

(fn `GetPlayerHorizontalDistance`
  (returns (ReturnValue :type "Float (double-precision)"))
  (return 0.0))

(fn `GetPlayerHorizontalDistance_0`
  (returns (ReturnValue :type "Float (double-precision)"))
  (bind (_returnvalue_x _returnvalue_y) (`KismetMathLibrary.BreakVector` (`self.K2_GetActorLocation`)))
  (bind (_returnvalue_x_2 _returnvalue_y_2) (`KismetMathLibrary.BreakVector` (`self.K2_GetActorLocation` (`GameplayStatics.GetPlayerPawn` 0))))
  (return (`KismetMathLibrary.Distance2D` (`KismetMathLibrary.MakeVector2D` _returnvalue_x _returnvalue_y) (`KismetMathLibrary.MakeVector2D` _returnvalue_x_2 _returnvalue_y_2))))

(fn `UserConstructionScript`)