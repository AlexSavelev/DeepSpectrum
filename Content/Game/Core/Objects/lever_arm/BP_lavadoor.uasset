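; Lava door obstacle that opens once every pressure plate in its NeedPlate array is switched on.
; Tick counts active Bp_plate entries and, when all are on, destroys the lava pipe mesh and trigger box, guarded by a Sep flag.
; Overlapping the box creates a How_open_door hint widget, which is only hidden on exit, so each new overlap creates another.
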(event `self.ReceiveTick`
  (params (DeltaSeconds :type "Float (single-precision)"))
  (bind _need_plate (`self.need_plate`))
  (for _array_element _need_plate
    (bind _asbp_plate (cast `/Game/Game/Core/Objects/lever_arm/Bp_plate` _array_element))
    (if (`/Game/Game/Core/Objects/lever_arm/Bp_plate.On/off` _asbp_plate)
      (set `self.click` (+ (`self.click`) 1))))
  (if (== (`KismetArrayLibrary.Array_Length` _need_plate) (`self.click`))
    (if (`self.sep`)
      (`ActorComponent.K2_DestroyComponent` (`self.SM_Dungeon_Pipes_Lava01`))
      (`ActorComponent.K2_DestroyComponent` (`self.Box`))
      (set `self.sep` false)
      (set `self.click` 0 :!label _label))
    (else
      (goto _label))))

(event `self.Box.OnComponentBeginOverlap`
  (params (OverlappedComponent :type "PrimitiveComponent Object Reference") (OtherActor :type "Actor Object Reference") (OtherComp :type "PrimitiveComponent Object Reference") (OtherBodyIndex :type Integer) (bFromSweep :type Boolean) (SweepResult :type "HitResult Structure (by ref)"))
  (bind _returnvalue (`|CreateWidget` "/Game/Game/Core/Widgets/how_open_door.how_open_door_C"))
  (set `self.door` _returnvalue)
  (`UserWidget.AddToViewport` _returnvalue 0))

(event `self.Box.OnComponentEndOverlap`
  (params (OverlappedComponent :type "PrimitiveComponent Object Reference") (OtherActor :type "Actor Object Reference") (OtherComp :type "PrimitiveComponent Object Reference") (OtherBodyIndex :type Integer))
  (`Widget.SetVisibility` (`self.door`) "Hidden"))

(fn `UserConstructionScript`)