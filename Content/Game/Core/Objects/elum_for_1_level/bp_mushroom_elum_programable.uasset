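; Programmable mushroom light whose "light_turn" and "Condition" programs decide when it turns on or off.
; OnUpdate caches both programs; Player applies "Always" at once, otherwise arms Sphere3, sized by the argument, to switch when the player enters.
; Entering Sphere and leaving the smaller Sphere1 adjust light counters on BPCHAR_driada and BP_ThirdPersonCharacter.
; Switching only toggles visibility of the light and three spheres, leaving collision untouched.
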(event `self.Player`
  (`|ExecutionSequence`
    (:`then_0`
      (if (and (== (`self.state of light`) "light_turn_of") (== (`self.condition`) "Always"))
        (`self.Visibity Of on/off` false)
        (set `self.set_tick` false :!label _label)
        (elif (and (== (`self.state of light`) "light_turn_on") (== (`self.condition`) "Always"))
          (`self.Visibity Of on/off` true)
          (goto _label)
          (else
            (`SphereComponent.SetSphereRadius` (`self.Sphere3`) (`KismetStringLibrary.Conv_StringToDouble` (`KismetTextLibrary.Conv_TextToString` (`self.argument`))) true)
            (set `self.set_tick` true)))))))

(event `self.OnUpdate`
  (bind _programs (break `/Game/Game/Core/Objects/Programmable/Structs/Data/S_POData` (`self.Programs`)))
  (bind _value (`BlueprintMapLibrary.Map_Find` _programs "Condition"))
  (set `self.argument` (`.Argument_9_554FC57544DA74CD8B7190AAC4106B00` (break `/Game/Game/Core/Objects/Programmable/Structs/Data/S_POScript` _value)))
  (bind _output_get (set `self.condition` (break `/Game/Game/Core/Objects/Programmable/Structs/Data/S_POScript` _value)))
  (set `self.state of light` (break `/Game/Game/Core/Objects/Programmable/Structs/Data/S_POScript` (`BlueprintMapLibrary.Map_Find` _programs "light_turn"))))

(event `self.Sphere3.OnComponentBeginOverlap`
  (params (OverlappedComponent :type "PrimitiveComponent Object Reference") (OtherActor :type "Actor Object Reference") (OtherComp :type "PrimitiveComponent Object Reference") (OtherBodyIndex :type Integer) (bFromSweep :type Boolean) (SweepResult :type "HitResult Structure (by ref)"))
  (if (== OtherActor (`GameplayStatics.GetPlayerPawn` 0))
    (if (`self.set_tick`)
      (if (== (`self.state of light`) "light_turn_on")
        (`self.Visibity Of on/off` true)
        (else
          (`self.Visibity Of on/off` false))))))

(event `self.Overview`
  (`KismetSystemLibrary.PrintString` "Hello"))

(event `self.ReceiveBeginPlay`
  (bind _radius_of_light (`self.radius_of_light`))
  (`|ExecutionSequence`
    (:`then_0`
      (`LightComponent.SetLightColor` (`self.PointLight1`) (`KismetMathLibrary.Conv_ColorToLinearColor` (`self.Light Color`)) true)
      (`SphereComponent.SetSphereRadius` (`self.Sphere`) _radius_of_light true)
      (`SphereComponent.SetSphereRadius` (`self.Sphere1`) (- _radius_of_light 100.0) true)
      (`SphereComponent.SetSphereRadius` (`self.Sphere2`) (`self.nearest_position_of_light`) true)
      (`LocalLightComponent.SetAttenuationRadius` (`self.PointLight1`) (`self.radius_of_light`)))
    (:`then_1`
      (`parent.ReceiveBeginPlay`))))

(event `self.Sphere.OnComponentBeginOverlap`
  (params (OverlappedComponent :type "PrimitiveComponent Object Reference") (OtherActor :type "Actor Object Reference") (OtherComp :type "PrimitiveComponent Object Reference") (OtherBodyIndex :type Integer) (bFromSweep :type Boolean) (SweepResult :type "HitResult Structure (by ref)"))
  (`|ExecutionSequence`
    (:`then_0`
      (bind _asbpchar_driada (cast `/Game/Game/Core/Objects/driada/BPCHAR_driada` OtherActor))
      (set `/Game/Game/Core/Objects/driada/BPCHAR_driada.is_Light_turn_on` (+ (`/Game/Game/Core/Objects/driada/BPCHAR_driada.is_Light_turn_on` _asbpchar_driada) 1) _asbpchar_driada)
      (set `/Game/Game/Core/Objects/driada/BPCHAR_driada.actual_light` self _asbpchar_driada))
    (:`then_1`
      (bind _asbp_third_person_character (cast `/Game/Game/Core/Characters/BP_ThirdPersonCharacter` OtherActor))
      (bind _output_get (set `/Game/Game/Core/Characters/BP_ThirdPersonCharacter.light_turn_on` (+ (`/Game/Game/Core/Characters/BP_ThirdPersonCharacter.light_turn_on` _asbp_third_person_character) 1) _asbp_third_person_character))
      (`KismetSystemLibrary.PrintString` (`KismetStringLibrary.Conv_IntToString` _output_get)))))

(event `self.Sphere1.OnComponentEndOverlap`
  (params (OverlappedComponent :type "PrimitiveComponent Object Reference") (OtherActor :type "Actor Object Reference") (OtherComp :type "PrimitiveComponent Object Reference") (OtherBodyIndex :type Integer))
  (`|ExecutionSequence`
    (:`then_0`
      (bind _asbpchar_driada (cast `/Game/Game/Core/Objects/driada/BPCHAR_driada` OtherActor))
      (set `/Game/Game/Core/Objects/driada/BPCHAR_driada.is_Light_turn_on` (- (`/Game/Game/Core/Objects/driada/BPCHAR_driada.is_Light_turn_on` _asbpchar_driada) 1) _asbpchar_driada)
      (set `/Game/Game/Core/Objects/driada/BPCHAR_driada.actual_light` self _asbpchar_driada))
    (:`then_1`
      (bind _asbp_third_person_character (cast `/Game/Game/Core/Characters/BP_ThirdPersonCharacter` OtherActor))
      (bind _output_get (set `/Game/Game/Core/Characters/BP_ThirdPersonCharacter.light_turn_on` (- (`/Game/Game/Core/Characters/BP_ThirdPersonCharacter.light_turn_on` _asbp_third_person_character) 1) _asbp_third_person_character))
      (`KismetSystemLibrary.PrintString` (`KismetStringLibrary.Conv_IntToString` _output_get)))))

(event `self.Sphere1.OnComponentBeginOverlap`
  (params (OverlappedComponent :type "PrimitiveComponent Object Reference") (OtherActor :type "Actor Object Reference") (OtherComp :type "PrimitiveComponent Object Reference") (OtherBodyIndex :type Integer) (bFromSweep :type Boolean) (SweepResult :type "HitResult Structure (by ref)")))

(event `self.Sphere2.OnComponentBeginOverlap`
  (params (OverlappedComponent :type "PrimitiveComponent Object Reference") (OtherActor :type "Actor Object Reference") (OtherComp :type "PrimitiveComponent Object Reference") (OtherBodyIndex :type Integer) (bFromSweep :type Boolean) (SweepResult :type "HitResult Structure (by ref)"))
  (cast `/Game/Game/Core/Objects/driada/BPCHAR_driada` OtherActor))

(fn `UserConstructionScript`)

(fn `Visibity Of on/off`
  (params (`on/off` :type Boolean))
  (`SceneComponent.SetVisibility` (`self.Sphere`) `on/off` false)
  (`SceneComponent.SetVisibility` (`self.Sphere1`) `on/off` false)
  (`SceneComponent.SetVisibility` (`self.Sphere2`) `on/off` false)
  (`SceneComponent.SetVisibility` (`self.PointLight1`) `on/off` false))