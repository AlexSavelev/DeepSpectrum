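; BP_actor_ceiling_killer_volume is a kill volume that resets the player and nearby gameplay state when the character enters its box.
; On overlap it sets the character's LightTurnOn, then teleports them to their saved BPA_save actor, falling back to StartCord.
; It also returns every BPCHAR_driada to its start position.
; The mushroom reset is nested in that loop, so all BP_Mushrooms reset once per dryad.
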(event `self.Box.OnComponentBeginOverlap`
  (params (OverlappedComponent :type "PrimitiveComponent Object Reference") (OtherActor :type "Actor Object Reference") (OtherComp :type "PrimitiveComponent Object Reference") (OtherBodyIndex :type Integer) (bFromSweep :type Boolean) (SweepResult :type "HitResult Structure (by ref)"))
  (bind _asbp_third_person_character (cast `/Game/Game/Core/Characters/BP_ThirdPersonCharacter` OtherActor))
  (set `/Game/Game/Core/Characters/BP_ThirdPersonCharacter.light_turn_on` 1 _asbp_third_person_character)
  (bind _asbpa_save (cast `/Game/Game/Core/Objects/saves/BPA_save` (`/Game/Game/Core/Characters/BP_ThirdPersonCharacter.actual_save` _asbp_third_person_character))
    (:`then`
      (`self.K2_SetActorLocation` _asbp_third_person_character (`self.K2_GetActorLocation` _asbpa_save) false true))
    (:`CastFailed`
      (`self.K2_SetActorLocation` _asbp_third_person_character (`/Game/Game/Core/Characters/BP_ThirdPersonCharacter.start_cord` _asbp_third_person_character) false true)))
  (bind _outactors (`GameplayStatics.GetAllActorsOfClass` "/Game/Game/Core/Objects/driada/BPCHAR_driada.BPCHAR_driada_C"))
  (for _index (range (`KismetArrayLibrary.Array_Length` _outactors))
    (bind _output (`|GetArrayItem` _outactors _index))
    (`self.K2_SetActorLocation` _output (`/Game/Game/Core/Objects/driada/BPCHAR_driada.start_cord_Driad` _output) false false)
    (bind _outactors_2 (`GameplayStatics.GetAllActorsOfClass` "/Game/Game/Core/Objects/Programmable/BP_Mushroom.BP_Mushroom_C"))
    (for _index_2 (range (`KismetArrayLibrary.Array_Length` _outactors_2))
      (bind _asbp_mushroom (cast `/Game/Game/Core/Objects/Programmable/BP_Mushroom` (`|GetArrayItem` _outactors_2 _index_2)))
      (`/Game/Game/Core/Objects/Programmable/BP_Mushroom.mushroom_reset` _asbp_mushroom))))

(fn `UserConstructionScript`)