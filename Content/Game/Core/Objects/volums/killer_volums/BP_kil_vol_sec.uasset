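; Kill volume that sends the gravity third-person character back to its last save point when it overlaps the box.
; On overlap it moves the character to its active Bp_save_sec, or to its start coordinates if none is set.
; It then restores gravity to the save's stored direction, defaulting to Down, and zeroes capsule velocity.
; Gravity is set by absolute rotation on player 0's pawn; the delta-rotation branch is hard-coded off.
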(event `self.Box.OnComponentBeginOverlap`
  (params (OverlappedComponent :type "PrimitiveComponent Object Reference") (OtherActor :type "Actor Object Reference") (OtherComp :type "PrimitiveComponent Object Reference") (OtherBodyIndex :type Integer) (bFromSweep :type Boolean) (SweepResult :type "HitResult Structure (by ref)"))
  (bind _rootcomponent (`Actor.RootComponent` OtherActor))
  (bind _asbp_third_person_character_gravity (cast `/Game/Game/Core/Characters/BP_ThirdPersonCharacter_Gravity` OtherActor))
  (bind _actual_save (`/Game/Game/Core/Characters/BP_ThirdPersonCharacter_Gravity.actual_save` _asbp_third_person_character_gravity))
  (cast `/Game/Game/Core/Objects/volums/killer_volums/Bp_save_sec` _actual_save
    (:`then`
      (`SceneComponent.K2_SetWorldLocation` _rootcomponent (`SceneComponent.K2_GetComponentLocation` (`Actor.RootComponent` _actual_save)) false false))
    (:`CastFailed`
      (`SceneComponent.K2_SetWorldLocation` _rootcomponent (`/Game/Game/Core/Characters/BP_ThirdPersonCharacter_Gravity.start_cord` _asbp_third_person_character_gravity) false false)))
  (`self.chang_gravity`)
  (`PrimitiveComponent.SetPhysicsLinearVelocity` (`/Game/Game/Core/Characters/BP_ThirdPersonCharacter_Gravity.Capsule` _asbp_third_person_character_gravity) (0.0 0.0 0.0) false "None"))

(fn `chang_gravity`
  (bind _asbp_third_person_character_gravity (cast `/Game/Game/Core/Characters/BP_ThirdPersonCharacter_Gravity` (`GameplayStatics.GetPlayerPawn` 0))
    (:`then`
      (bind _asbp_save_sec (cast `/Game/Game/Core/Objects/volums/killer_volums/Bp_save_sec` (`/Game/Game/Core/Characters/BP_ThirdPersonCharacter_Gravity.actual_save` _asbp_third_person_character_gravity))
        (:`then`
          (set `self.Direction` (`/Game/Game/Core/Objects/volums/killer_volums/Bp_save_sec.dir` _asbp_save_sec)))
        (:`CastFailed`
          (set `self.Direction` "Down")))
      (set `self.Pawn` _asbp_third_person_character_gravity)
      (if false
        (`/Game/Game/Core/Characters/BP_ThirdPersonCharacter_Gravity.SetGravityByDeltaRotation` (`self.Pawn`) (`KismetMathLibrary.SelectRotator` (struct :`Pitch` 90.0) (struct :`Pitch` -90.0) (== (`self.Direction`) "Clockwise")) 10.0)
        (return)
        (else
          (`/Game/Game/Core/Characters/BP_ThirdPersonCharacter_Gravity.SetGravityByRotation` (`self.Pawn`) (select `int` (`KismetArrayLibrary.Array_Find` (`|MakeArray` "Up" "Down" "Front" "Back" :!type "Name") (`self.Direction`)) :`0` (struct :`Roll` 179.899994) :`1` (struct) :`2` (struct :`Pitch` -90.0) :`3` (struct :`Pitch` 90.0) :!type "Rotator Structure") 10.0)
          (return))))
    (:`CastFailed`
      (`KismetSystemLibrary.PrintString` "Gravity Changer works only with TPCh2 class!")
      (return))))

(fn `UserConstructionScript`)