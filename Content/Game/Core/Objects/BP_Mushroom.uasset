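; BP_Mushroom is a programmable mushroom object whose program is edited through an on-screen widget.
; On OnProgram, it shows the third-person character's MushroomProgramWidget, binds to its finish event and passes it the current Program and Limits.
; When the widget finishes, the mushroom stores the new program, calls OnFinishProgramming, then removes and unbinds the shared widget.
; BeginPlay and construction only defer to the parent class.
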(event `self.ReceiveBeginPlay`
  (`parent.ReceiveBeginPlay`))

(event `self.OnProgram`
  (bind _mushroomprogramwidget (`/Game/Game/Core/Characters/BP_ThirdPersonCharacter.MushroomProgramWidget` (`/Game/Game/Core/Functional/BPFL_Main.GetTPPCharacter`)))
  ;[1 1 1] Programming
  (`UserWidget.AddToViewport` _mushroomprogramwidget 0)
  (add `/Game/Game/Core/Objects/Mushroom/WBP_MushroomProgram.OnFinish` _mushroomprogramwidget (delegate `OnInterfaceFinished`))
  (`/Game/Game/Core/Objects/Mushroom/WBP_MushroomProgram.ProgramIt` _mushroomprogramwidget (`self.Program`) (`self.Limits`)))

(event `OnInterfaceFinished`
  (params (NewProgram :type "/Game/Game/Core/Objects/Mushroom/S_MushroomProgram Structure"))
  (bind _mushroomprogramwidget (`/Game/Game/Core/Characters/BP_ThirdPersonCharacter.MushroomProgramWidget` (`/Game/Game/Core/Functional/BPFL_Main.GetTPPCharacter`)))
  ;[1 1 1] Programming
  (set `self.Program` NewProgram)
  (`self.OnFinishProgramming`)
  (`Widget.RemoveFromParent` _mushroomprogramwidget)
  (remove `/Game/Game/Core/Objects/Mushroom/WBP_MushroomProgram.OnFinish` _mushroomprogramwidget (delegate `OnInterfaceFinished`)))

(fn `UserConstructionScript`
  (`parent.UserConstructionScript`))