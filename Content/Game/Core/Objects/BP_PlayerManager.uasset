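; BP_PlayerManager switches play between the player pawn and an overview pawn.
; On BeginPlay it caches the player pawn, classifies it by Blueprint class, spawns a BP_Overviewer and registers with the GameInstance.
; Overview mode configures the overviewer with spline, speed, trace length and location, possesses it and enables cursor and UI input.
; Player mode re-possesses the player with game-only input; both switches notify the GameInstance and fire mode-change calls.
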(event `self.ReceiveBeginPlay`
  (set `self.Player` (`GameplayStatics.GetPlayerPawn` 0))
  (`self.DefinePlayerClass`)
  (bind _returnvalue (`|SpawnActorFromClass` "/Game/Game/Core/Characters/BP_Overviewer.BP_Overviewer_C" (`KismetMathLibrary.MakeTransform` (0.0 0.0 0.0)) "Undefined" "OverrideRootScale" null self null))
  (set `self.Overviewer` _returnvalue)
  (`/Game/Game/Core/GI_Main.RegisterPlay` (`/Game/Game/Core/Functional/BPFL_Main.GameInstance`) self))

(event `SetGMOverviewer`
  (params (Spline :type "/Game/Game/Core/Cameras/BP_CameraSpline Object Reference") (Speed :type "Float (double-precision)") (TraceLength :type "Float (double-precision)") (Location :type "Vector Structure"))
  (bind _returnvalue (`GameplayStatics.GetPlayerController` 0))
  (`/Game/Game/Core/Characters/BP_Overviewer.Setup` (`self.Overviewer`) Spline Speed TraceLength Location)
  (set `self.bIsOverviewer` true)
  (`Controller.Possess` _returnvalue (`self.Overviewer`))
  (set `PlayerController.bShowMouseCursor` true _returnvalue)
  (`WidgetBlueprintLibrary.SetInputMode_GameAndUIEx` _returnvalue null)
  (`/Game/Game/Core/GI_Main.OnOverviewer` (`/Game/Game/Core/Functional/BPFL_Main.GameInstance`))
  (`/Game/Game/Core/Characters/BP_Overviewer.OnOverview` (`self.Overviewer`))
  (`self.OnChangeGameModeOverview`) ; For Programming Objects
)

(event `SetGMPlayer`
  (bind _returnvalue (`GameplayStatics.GetPlayerController` 0))
  (set `self.bIsOverviewer` false)
  (`Controller.Possess` _returnvalue (`self.Player`))
  (`WidgetBlueprintLibrary.SetInputMode_GameOnly` _returnvalue)
  (`/Game/Game/Core/GI_Main.OnPlayer` (`/Game/Game/Core/Functional/BPFL_Main.GameInstance`))
  (`self.OnChangeGameModePlayer`))

(fn `DefinePlayerClass`
  (set `self.PlayerClass` (select `bool` (== (`GameplayStatics.GetObjectClass` (`self.Player`)) "/Game/Game/Core/Characters/BP_ThirdPersonCharacter.BP_ThirdPersonCharacter_C") :`false` "NewEnumerator1" :`true` "NewEnumerator0" :!type "/Game/Game/Core/Characters/E_PlayerClass Enum"))
  (return))

(fn `UserConstructionScript`)