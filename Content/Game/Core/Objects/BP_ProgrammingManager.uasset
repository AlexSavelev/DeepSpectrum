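; BP_ProgrammingManager switches the player between third-person character control and an overview mode using a BP_Overviewer pawn.
; On BeginPlay it caches the character and spawns the overviewer with itself as manager.
; SetGMOverviewer configures the overviewer from a spline, speed, trace length and location, possesses it and shows the cursor.
; SetGMPlayer re-possesses the character with game-only input; each switch calls a mode-change notification.
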(event `self.ReceiveBeginPlay`
  (bind _asbp_third_person_character (cast `/Game/Game1/Core/Characters/BP_ThirdPersonCharacter` (`GameplayStatics.GetPlayerCharacter` 0)))
  (set `self.Player` _asbp_third_person_character)
  (bind _returnvalue (`|SpawnActorFromClass` "/Game/Game/Core/Characters/BP_Overviewer.BP_Overviewer_C" (`KismetMathLibrary.MakeTransform` (0.0 0.0 0.0)) "Undefined" "OverrideRootScale" null self null))
  (set `self.Overviewer` _returnvalue))

(event `SetGMOverviewer`
  (params (Spline :type "/Game/Game/Core/Cameras/BP_CameraSpline Object Reference") (Speed :type "Float (double-precision)") (TraceLength :type "Float (double-precision)") (Location :type "Vector Structure"))
  (bind _returnvalue (`GameplayStatics.GetPlayerController` 0))
  (`/Game/Game/Core/Characters/BP_Overviewer.Setup` (`self.Overviewer`) Spline Speed TraceLength Location)
  (set `self.PlayerLocation` (`self.K2_GetActorLocation`))
  (set `self.bIsOverviewer` true)
  (`Controller.Possess` _returnvalue (`self.Overviewer`))
  (set `PlayerController.bShowMouseCursor` true _returnvalue)
  (`WidgetBlueprintLibrary.SetInputMode_GameAndUIEx` _returnvalue null)
  (`/Game/Game/Core/Characters/BP_Overviewer.OnOverview` (`self.Overviewer`))
  (`self.OnChangeGameModeOverview`))

(event `SetGMPlayer`
  (bind _returnvalue (`GameplayStatics.GetPlayerController` 0))
  (bind _outactors (`GameplayStatics.GetAllActorsOfClass` "/Game/Game1/Core/Characters/BP_ThirdPersonCharacter.BP_ThirdPersonCharacter_C"))
  (bind _asbp_third_person_character (cast `/Game/Game1/Core/Characters/BP_ThirdPersonCharacter` (`|GetArrayItem` _outactors)))
  (set `self.Player` _asbp_third_person_character)
  (`KismetSystemLibrary.PrintString` "Hello")
  (set `self.bIsOverviewer` false)
  (`Controller.Possess` _returnvalue (`self.Player`))
  (`WidgetBlueprintLibrary.SetInputMode_GameOnly` _returnvalue)
  (`self.OnChangeGameModePlayer`))

(fn `UserConstructionScript`)