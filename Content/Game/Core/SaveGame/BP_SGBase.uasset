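; BP_SGBase is a base save-game object holding play state, map, player transform, gravity, light, temperature, completed levels and a description struct.
; SetLocation and SetGravitation are setters for the transform and gravity fields.
; FillFromTemplate seeds a save from the map's DT_MapSaveTemplates row, using both setters and stamping the passed date, row title and completed levels.
; A missing row leaves the object unchanged.
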(fn `FillFromTemplate`
  (params (Map :type Name) (Date :type "DateTime Structure") (CompletedLevels :type "Array of Boolean"))
  (bind _returnvalue (`|GetDataTableRow` "/Game/Game/Core/SaveGame/DT_MapSaveTemplates.DT_MapSaveTemplates" Map)
    (:`then`
      (bind (_title _playerlocation _playerrotation _playstate _gravityrotation _gravityforce _lightturnon _temperature) (break `/Game/Game/Core/SaveGame/Structs/S_SaveGameTemplate` _returnvalue))
      (setmembers `/Game/Game/Core/SaveGame/Structs/S_SaveGameDesc` :`StructRef` (`self.Desc`) :`Date` Date :`DisplayName` _title)
      (`self.SetLocation` _playstate Map _playerlocation _playerrotation)
      (`self.SetGravitation` _gravityrotation _gravityforce)
      (set `self.LightTurnOn` _lightturnon)
      (set `self.Temperature` _temperature)
      (set `self.CompletedLevels` CompletedLevels)
      (return))
    (:`RowNotFound`
      (return))))

(fn `SetGravitation`
  (params (Rotation :type "Rotator Structure") (Force :type "Float (double-precision)"))
  (set `self.GravityRotation` Rotation)
  (set `self.GravityForce` Force)
  (return))

(fn `SetLocation`
  (params (State :type "/Game/Game/Core/Characters/E_GameState Enum" :default "NewEnumerator0") (Level :type Name) (Location :type "Vector Structure") (Rotation :type "Rotator Structure"))
  (set `self.PlayState` State)
  (set `self.Map` Level)
  (set `self.Location` Location)
  (set `self.Rotation` Rotation)
  (return))