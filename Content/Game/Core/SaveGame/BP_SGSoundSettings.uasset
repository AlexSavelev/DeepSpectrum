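; BP_SGSoundSettings is a save-game Blueprint that holds the sound volume settings: a multiply volume plus music, SFX and voice volumes.
; GetAsArray packs the four values into an array in a fixed order, and PutAsArray writes an array back into them by the same indices.
; PutAsArray does no length check or clamping, so callers depend on that index order.
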(fn `GetAsArray`
  (returns (ReturnValue :type "Array of Float (double-precision)"))
  (return (`|MakeArray` (`self.MultiplyVolume`) (`self.MusicVolume`) (`self.SFXVolume`) (`self.VoiceVolume`))))

(fn `PutAsArray`
  (params (SoundVolumes :type "Array of Float (double-precision)"))
  (set `self.MultiplyVolume` (`|GetArrayItem` SoundVolumes))
  (set `self.MusicVolume` (`|GetArrayItem` SoundVolumes 1))
  (set `self.SFXVolume` (`|GetArrayItem` SoundVolumes 2))
  (set `self.VoiceVolume` (`|GetArrayItem` SoundVolumes 3))
  (return))